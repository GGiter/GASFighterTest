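; Player character with camera-relative Enhanced Input movement, light and heavy attacks, a GAS roll and sword/fist combat-data switching.
; Each tick sets max speed from gait and a strafe-angle curve, switches rotation rate when falling, and blends camera settings between close combat and far styles.
; Gait resolves only to Run while sprint is held, otherwise Walk; Sprint is never returned and analog input has no effect on it.
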(event Input|EnhancedActionEvents|EnhancedInputActionIA_Move
  (params (ActionValue :type Vector%202D%20Structure) (ElapsedSeconds :type Float%20%28double-precision%29) (TriggeredSeconds :type Float%20%28double-precision%29) (InputAction :type Input%20Action%20Object%20Reference :default "/Game/Input/IA_Move.IA_Move"))
  (bind _returnvalue (Pawn|GetControlRotation :!class /Script/Engine.Pawn))
  (bind (_x _y) (Math|Vector2D|BreakVector2D ActionValue))
  ;[1 1 1] Inputs
  (if (not (Class|MKOICharacter|IsDead))
    (Pawn|Input|AddMovementInput (Math|Vector|GetRightVector (Math|Rotator|MakeRotator 0.0 0.0 (.yaw _returnvalue))) _x false)
    (Pawn|Input|AddMovementInput (Math|Vector|GetForwardVector (Math|Rotator|MakeRotator 0.0 0.0 (.yaw _returnvalue))) _y false)))

(event Input|EnhancedActionEvents|EnhancedInputActionIA_Walk
  (params (ActionValue :type Boolean) (ElapsedSeconds :type Float%20%28double-precision%29) (TriggeredSeconds :type Float%20%28double-precision%29) (InputAction :type Input%20Action%20Object%20Reference :default "/Game/Input/IA_Walk.IA_Walk"))
  ;[1 1 1] Inputs
  (if (not (Class|MKOICharacter|IsDead))
    (if (not (Variables|Movement|GetWantsToSprint))
      (Variables|Movement|SetWantsToWalk (not (Variables|Movement|GetWantsToWalk))))))

(event Input|EnhancedActionEvents|EnhancedInputActionIA_Look
  (params (ActionValue :type Vector%202D%20Structure) (ElapsedSeconds :type Float%20%28double-precision%29) (TriggeredSeconds :type Float%20%28double-precision%29) (InputAction :type Input%20Action%20Object%20Reference :default "/Game/Input/IA_Look.IA_Look"))
  ;[1 1 1] Inputs
  (if (not (Class|MKOICharacter|IsDead))
    (Pawn|Input|AddControllerYawInput (.x ActionValue))
    (Pawn|Input|AddControllerPitchInput (.y ActionValue))))

(event Input|EnhancedActionEvents|EnhancedInputActionIA_Look_Gamepad
  (params (ActionValue :type Vector%202D%20Structure) (ElapsedSeconds :type Float%20%28double-precision%29) (TriggeredSeconds :type Float%20%28double-precision%29) (InputAction :type Input%20Action%20Object%20Reference :default "/Game/Input/IA_Look_Gamepad.IA_Look_Gamepad"))
  (bind _returnvalue (Utilities|Time|GetWorldDeltaSeconds))
  (bind _returnvalue_2 (* ActionValue _returnvalue))
  ;[1 1 1] Inputs
  (if (not (Class|MKOICharacter|IsDead))
    (Pawn|Input|AddControllerYawInput (.x _returnvalue_2))
    (Pawn|Input|AddControllerPitchInput (.y _returnvalue_2))))

(event Input|EnhancedActionEvents|EnhancedInputActionIA_Roll
  (params (ActionValue :type Boolean) (ElapsedSeconds :type Float%20%28double-precision%29) (TriggeredSeconds :type Float%20%28double-precision%29) (InputAction :type Input%20Action%20Object%20Reference :default "/Game/Input/IA_Roll.IA_Roll"))
  ;[1 1 1] Inputs
  (Abilities|TryActivateAbilitybyClass (Variables|Default|GetAbilitySystemComponent) "/Game/Blueprints/Abilities/GA_RollAbility.GA_RollAbility_C" true))

(event Input|EnhancedActionEvents|EnhancedInputActionIA_Sprint
  (params (ActionValue :type Boolean) (ElapsedSeconds :type Float%20%28double-precision%29) (TriggeredSeconds :type Float%20%28double-precision%29) (InputAction :type Input%20Action%20Object%20Reference :default "/Game/Input/IA_Sprint.IA_Sprint"))
  ;[1 1 1] Inputs
  (if (not (Class|MKOICharacter|IsDead))
    (Variables|Movement|SetWantsToSprint ActionValue)
    (Variables|Movement|SetWantsToWalk false)))

(event Input|EnhancedActionEvents|EnhancedInputActionIA_LightAttack
  (params (ActionValue :type Boolean) (ElapsedSeconds :type Float%20%28double-precision%29) (TriggeredSeconds :type Float%20%28double-precision%29) (InputAction :type Input%20Action%20Object%20Reference :default "/Game/Input/IA_LightAttack.IA_LightAttack"))
  ;[1 1 1] Inputs
  (Class|MKOICharacter|PerformLightAttack))

(event Input|EnhancedActionEvents|EnhancedInputActionIA_HeavyAttack
  (params (ActionValue :type Boolean) (ElapsedSeconds :type Float%20%28double-precision%29) (TriggeredSeconds :type Float%20%28double-precision%29) (InputAction :type Input%20Action%20Object%20Reference :default "/Game/Input/IA_HeavyAttack.IA_HeavyAttack"))
  ;[1 1 1] Inputs
  (Class|MKOICharacter|PerformHeavyAttack))

(event Input|EnhancedActionEvents|EnhancedInputActionIA_SwtichWeapon
  (params (ActionValue :type Boolean) (ElapsedSeconds :type Float%20%28double-precision%29) (TriggeredSeconds :type Float%20%28double-precision%29) (InputAction :type Input%20Action%20Object%20Reference :default "/Game/Input/IA_SwtichWeapon.IA_SwtichWeapon"))
  ;[1 1 1] Inputs
  (if (not (Class|MKOICharacter|IsDead))
    (Utilities|FlowControl|FlipFlop
      (:A
        (Class|MKOICharacter|ChangeWeaponDataAsset "/Game/DataAssets/DA_SwordCombatData.DA_SwordCombatData"))
      (:B
        (Class|MKOICharacter|ChangeWeaponDataAsset "/Game/DataAssets/DA_FistCombatData.DA_FistCombatData")))))

(event EventPossessed
  (params (NewController :type Controller%20Object%20Reference))
  (Utilities|IsValid NewController
    (:Is%20Valid
      (bind _asplayer_controller (Utilities|Casting|CastToPlayerController NewController))
      (Input|AddMappingContext (PlayerController|LocalPlayerSubsystems|GetEnhancedInputLocalPlayerSubsystem _asplayer_controller) "/Game/Input/IMC_Setup.IMC_Setup" 0 "(bIgnoreAllPressedKeysUntilRelease=True,bForceImmediately=False,bNotifyUserSettings=False)"))))

(event EventTick
  (params (DeltaSeconds :type Float%20%28single-precision%29))
  (CallFunction|UpdateMovement)
  (CallFunction|UpdateRotation)
  (CallFunction|UpdateCamera true))

(fn ConstructionScript)

(fn UpdateMovement
  (Utilities|FlowControl|Sequence
    (:then_0
      (Variables|Movement|SetGait (CallFunction|GetDesiredGait)))
    (:then_1
      (bind _output_get (Variables|/Script/Engine.CharacterMovementComponent|SetMaxWalkSpeed (Variables|Character|GetCharacterMovement) (CallFunction|CalculateMaxSpeed)))
      (Variables|/Script/Engine.CharacterMovementComponent|SetMaxWalkSpeedCrouched (Variables|Character|GetCharacterMovement) _output_get))))

(fn UpdateCamera
  (params (Interpolate :type Boolean))
  (bind _cameradistancemultiplier (Variables|Camera|GetCameraDistanceMultiplier))
  (bind _bisincombat (Variables|Default|GetbIsInCombat))
  (bind _camstyle_far (Variables|Camera|GetCamStyle_Far))
  (bind _camstyle_close (Variables|Camera|GetCamStyle_Close))
  (bind _returnvalue (select _bisincombat _camstyle_close _camstyle_far))
  (bind (_springarmlength _socketoffset _translationlagspeed _fieldofview _transitionspeed) (Utilities|Struct|BreakS_SimpleCameraParams _returnvalue))
  (Variables|Camera|SetTargetCameraParams (Utilities|Struct|MakeS_SimpleCameraParams (* _springarmlength _cameradistancemultiplier) (* _socketoffset _cameradistancemultiplier) (Math|Float|SelectFloat _translationlagspeed -1.0 Interpolate) _fieldofview (Math|Float|SelectFloat _transitionspeed -1.0 Interpolate)))
  (bind _output_get (Variables|/Script/Engine.CameraComponent|SetFieldOfView (Variables|Default|GetCamera) (Math|Interpolation|FInterpTo (stale _output_get) (.fieldofview (Variables|Camera|GetTargetCameraParams)) (Utilities|Time|GetWorldDeltaSeconds) (.transitionspeed (Variables|Camera|GetTargetCameraParams)))))
  (bind _output_get_2 (Variables|/Script/Engine.SpringArmComponent|SetTargetArmLength (Variables|Default|GetSpringArm) (Math|Interpolation|FInterpTo (stale _output_get_2) (.springarmlength (Variables|Camera|GetTargetCameraParams)) (Utilities|Time|GetWorldDeltaSeconds) (.transitionspeed (Variables|Camera|GetTargetCameraParams)))))
  (bind _output_get_3 (Variables|/Script/Engine.SpringArmComponent|SetCameraLagSpeed (Variables|Default|GetSpringArm) (Math|Interpolation|FInterpTo (stale _output_get_3) (.translationlagspeed (Variables|Camera|GetTargetCameraParams)) (Utilities|Time|GetWorldDeltaSeconds) (.transitionspeed (Variables|Camera|GetTargetCameraParams)))))
  (bind _output_get_4 (Variables|/Script/Engine.SpringArmComponent|SetSocketOffset (Variables|Default|GetSpringArm) (Math|Interpolation|VInterpTo (stale _output_get_4) (.socketoffset (Variables|Camera|GetTargetCameraParams)) (Utilities|Time|GetWorldDeltaSeconds) (.transitionspeed (Variables|Camera|GetTargetCameraParams))))))

(fn UpdateRotation
  (if (AI|Components|NavMovement|IsFalling (Variables|Character|GetCharacterMovement))
    (Variables|/Script/Engine.CharacterMovementComponent|SetRotationRate (Variables|Character|GetCharacterMovement) "0.000000,200.000000,0.000000")
    (else
      (Variables|/Script/Engine.CharacterMovementComponent|SetRotationRate (Variables|Character|GetCharacterMovement) "0.000000,-1.000000,0.000000"))))

(fn GetDesiredGait
  (Variables|Movement|SetFullMovementInput (>= (Math|Vector2D|Vector2DLength (Input|EnhancedActionValues|GetIA_Move)) (Variables|Movement|GetAnalogWalk/RunThreshold)))
  (if (Variables|Movement|GetWantsToSprint)
    (if (Variables|Movement|GetFullMovementInput)
      (return "Run")
      (else
        (return "Run")))
    (elif (Variables|Movement|GetWantsToWalk)
      (return "Walk")
      (elif (Variables|Movement|GetFullMovementInput)
        (return "Walk")
        (else
          (return "Walk"))))))

(fn CalculateMaxSpeed
  (bind _runspeeds (Variables|Movement|GetRunSpeeds))
  (bind _sprintspeeds (Variables|Movement|GetSprintSpeeds))
  (bind _charactermovement (Variables|Character|GetCharacterMovement))
  (bind _crouchspeeds (Variables|Movement|GetCrouchSpeeds))
  (bind _gait (Variables|Movement|GetGait))
  (bind _walkspeeds (Variables|Movement|GetWalkSpeeds))
  (bind _returnvalue (AI|Components|NavMovement|IsCrouching _charactermovement))
  (bind _returnvalue_2 (Utilities|Select :Index _gait :Walk _walkspeeds :Run _runspeeds :Sprint _sprintspeeds))
  (bind _returnvalue_3 (select _returnvalue _crouchspeeds _returnvalue_2))
  (Variables|Movement|SetStrafeSpeedMap (Math|Curves|GetFloatValue (Variables|Movement|GetStrafeSpeedMapCurve) (Math|Float|Absolute(Float) (Class|KismetAnimationLibrary|CalculateDirection (Variables|/Script/Engine.MovementComponent|GetVelocity (Variables|Character|GetCharacterMovement)) (Transformation|GetActorRotation)))))
  (return (Math|Float|SelectFloat (Math|Float|MapRangeClamped (Variables|Movement|GetStrafeSpeedMap) 0.0 1.0 (.x _returnvalue_3) (.y _returnvalue_3)) (Math|Float|MapRangeClamped (Variables|Movement|GetStrafeSpeedMap) 1.0 2.0 (.y _returnvalue_3) (.z _returnvalue_3)) (< (Variables|Movement|GetStrafeSpeedMap) 1.0))))